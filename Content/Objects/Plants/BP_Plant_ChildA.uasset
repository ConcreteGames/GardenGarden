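; BP_Plant_ChildA is a plant variant that sets its own index, anchor scale and growth, seeding and water stats in the construction script.
; On BeginPlay it scans plant visuals overlapping its local visual's sphere.
; It destroys itself if one with index 0 or 4 lies within a radius derived from that visual's sphere scale.
; Any other valid overlap toggles the visibility of its Visual component.
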(event EventBeginPlay
  (|CallParentFunction)
  (for _array_element (Collision|GetOverlappingActors (Variables|/Game/Objects/Plants/BP_PlantVisual_Parent.BP_PlantVisual_Parent_C|GetSphere (.AsBP%20Plant%20Visual%20Parent (Utilities|Casting|CastToBP_PlantVisual_Parent (Variables|Default|GetLocalVIsual)))) "/Game/Objects/Plants/BP_PlantVisual_Parent.BP_PlantVisual_Parent_C" :!class /Script/Engine.PrimitiveComponent)
    (Utilities|IsValid _array_element
      (:Is%20Valid
        (bind _asbp_plant_visual_parent (Utilities|Casting|CastToBP_PlantVisual_Parent _array_element))
        (if (and (or (== (Variables|/Game/Objects/Plants/BP_PlantVisual_Parent.BP_PlantVisual_Parent_C|GetPlantIndex _asbp_plant_visual_parent) 0) (== (Variables|/Game/Objects/Plants/BP_PlantVisual_Parent.BP_PlantVisual_Parent_C|GetPlantIndex _asbp_plant_visual_parent) 4)) (< (Math|Vector|VectorLength (- (Transformation|GetActorLocation) (Transformation|GetActorLocation _asbp_plant_visual_parent))) (* (* (Variables|/Game/Objects/Plants/BP_PlantVisual_Parent.BP_PlantVisual_Parent_C|GetSphereScale _asbp_plant_visual_parent) 1.5) 5e+01)))
          (Variables|Default|SetToDestroy true)
          (else
            (Rendering|ToggleVisibility (Variables|Default|GetVisual) false))))))
  (if (Variables|Default|GetToDestroy)
    (Actor|DestroyActor)))

(event Collision|EventActorBeginOverlap
  (params (OtherActor :type Actor%20Object%20Reference)))

(event EventTick
  (params (DeltaSeconds :type Float%20%28single-precision%29))
  (|CallParentFunction DeltaSeconds))

(fn ConstructionScript
  (|CallParentFunction)
  (Variables|Default|SetPlantIndex 0)
  (Transformation|SetRelativeScale3D (Variables|Default|GetAnchorScaleTemp) "1.500000,1.500000,0.300000")
  (CallFunction|SetValues 1e+04 999999999.0 0.0 0 0.5 2.5 0.1 false -5e+03 0.3 false))