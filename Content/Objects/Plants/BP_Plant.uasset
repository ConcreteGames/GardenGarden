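; Plant master actor with a draining lifespan: watering restores life and speeds up its bud, which periodically spawns seeds.
; BeginPlay spawns tiled visual copies of the plant, which scale and tint with its life.
; Tick pulls overlapping same-index plants together to fuse into a new seed, drains life near other kinds, and randomly spawns weeds.
; Watering-type plants also fire drops from every copy on a life-driven timeline, gaining nozzles over time.
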(event Custom|Water
  (bind _sfx_water (Variables|Default|GetSFX_Water))
  (Variables|Default|SetLifeRemaining (select (> (+ (Variables|Default|GetLifeRemaining) (Variables|Default|GetWaterAddTime)) (Variables|Default|GetLifeMax)) (Variables|Default|GetLifeMax) (+ (Variables|Default|GetLifeRemaining) (Variables|Default|GetWaterAddTime))))
  (Bud|BudFeed)
  ;[1 1 1] SFX Suck water
  (if (not (Audio|Components|Audio|IsPlaying _sfx_water))
    (Audio|Components|Audio|Play _sfx_water 0.0)))

(event Custom|StartWatering
  (bind _liferemaining (Variables|Default|GetLifeRemaining))
  (bind _lifemax (Variables|Default|GetLifeMax))
  (bind _crv_wateringbylife (Variables|Water|GetCRV_WateringByLife))
  (bind _returnvalue (/ _liferemaining _lifemax))
  (bind _returnvalue_2 (Math|Curves|GetFloatValue _crv_wateringbylife _returnvalue))
  (Utilities|FlowControl|Sequence
    (:then_0
      (Components|Timeline|SetTimelineLength (Variables|Default|GetWateringFrequency) (* _returnvalue_2 0.2))
      (Timeline|WateringFrequency PlayFromStart
        (:Finished
          (CallFunction|WateringPlant)
          (Components|Timeline|SetTimelineLength (Variables|Default|GetWateringFrequency) (* _returnvalue_2 (Variables|Water|GetWateringRate)))
          (Timeline|WateringFrequency PlayFromStart))))
    (:then_1
      (Utilities|FlowControl|Delay 1.2e+02)
      (Variables|Water|SetNumberOfDick 2)
      (Utilities|FlowControl|Delay 2.4e+02)
      (Variables|Water|SetNumberOfDick 3))))

(event Custom|UpdateVisualEvent
  (params (InputPin :type Float%20%28single-precision%29))
  (bind _liferemaining (Variables|Default|GetLifeRemaining))
  (bind _lifemax (Variables|Default|GetLifeMax))
  (bind _returnvalue (/ _liferemaining _lifemax))
  (bind _returnvalue_2 (* _returnvalue 0.75))
  (bind _returnvalue_3 (+ 0.25 _returnvalue_2))
  (Default|UpdateTransform (Variables|Default|GetVisuals) (Math|Transform|MakeTransform (Transformation|GetActorLocation) (Transformation|GetActorRotation) (Math|Vector|MakeVector _returnvalue_3 _returnvalue_3 _returnvalue_3)) (Variables|Bud|GetBudScale))
  ;[1 1 1] Feedback more life
  (if (Audio|Components|Audio|IsPlaying (Variables|Default|GetFeedbackLifeSecu))
    ;;[1 1 1] If Always 1, reinit secu
    (if (and (> (Variables|Default|GetPreviousLifeGain) 0.0) (> InputPin 0.0))
      ;;[1 1 1] If not 0, launch secu
      ;; to always have an at least 1 second feedback
      (Components|Timeline|PlayfromStart (Variables|Default|GetFeedbackLifeSecu) :!label _label))
    (else
      (Default|UpdateMaterialParams :self (Variables|Default|GetVisuals) :LifeState InputPin)
      (bind _output_get (Variables|Default|SetPreviousLifeGain InputPin))
      (if (> _output_get 0.0)
        (goto _label)))))

(event EventBeginPlay
  (bind _lifemax (Variables|Default|GetLifeMax))
  ;[0.2251 1 0] BEGIN PLAY
  (|CallParentFunction)
  (CallFunction|ReplicatePlant)
  (Bud|InitSpawnSeedTimer)
  (Variables|Default|SetLifeRemaining _lifemax)
  (Variables|Default|SetCurrentLife _lifemax)
  (if (Variables|Default|GetIsWateringPlant)
    (CallFunction|StartWatering)))

(event EventTick
  (params (DeltaSeconds :type Float%20%28single-precision%29))
  ;[0.01803 1 0] EVENT TICK
  (CallFunction|TestOtherPlantProximity)
  (Bud|BudGrowing)
  (Bud|BudUpdateScaleValue)
  (CallFunction|Weed)
  (bind _newlife (CallFunction|UpdateLife))
  (CallFunction|Death _newlife)
  (bind _lifegain (CallFunction|LifeGain))
  (CallFunction|UpdateVisualEvent _lifegain))

(fn ConstructionScript
  (|CallParentFunction))

(fn UpdateLife
  (bind _output_get (Variables|Default|SetLifeRemaining (- (Variables|Default|GetLifeRemaining) (Utilities|Time|GetWorldDeltaSeconds))))
  (return _output_get))

(fn ScaleVisualbyLife
  (bind _liferemaining (Variables|Default|GetLifeRemaining))
  (bind _lifemax (Variables|Default|GetLifeMax))
  (bind _returnvalue (/ _liferemaining _lifemax))
  (bind _returnvalue_2 (* _returnvalue 0.75))
  (bind _returnvalue_3 (+ 0.25 _returnvalue_2))
  (Transformation|SetRelativeScale3D (Variables|Default|GetVisual) (Math|Vector|MakeVector _returnvalue_3 _returnvalue_3 _returnvalue_3)))

(fn Death
  (params (A :type Float%20%28single-precision%29))
  (if (< A 0.0)
    (Actor|SetLifeSpan (Variables|Default|GetVisuals) 0.01)
    (Actor|DestroyActor)))

(fn SpawnSeed
  (Transformation|SetRelativeRotation (Variables|Default|GetAnchorRotation) (Math|Rotator|MakeRotator 0.0 0.0 (Math|Random|RandomFloatinRange 0.0 3.6e+02)) false false)
  (Game|SpawnActorfromClass "/Game/Objects/BP_Seed.BP_Seed_C" (Math|Transform|MakeTransform (+ (Transformation|GetActorLocation) (* (Transformation|GetActorUpVector) 2e+02)) (Transformation|GetWorldRotation (Variables|Default|GetSpawnSeedDirection)) "1,1,1") "Undefined" 0 false 1 false 0))

(fn TestOtherPlantProximity
  (bind _returnvalue (Transformation|GetActorLocation))
  (bind _plantindex (Variables|Default|GetPlantIndex))
  (if (Variables|Default|GetIsActive)
    (for _array_element (Collision|GetOverlappingActors (Variables|/Game/Objects/Plants/BP_PlantVisual_Parent.BP_PlantVisual_Parent_C|GetSphere (.AsBP%20Plant%20Visual%20Parent (Utilities|Casting|CastToBP_PlantVisual_Parent (Variables|Default|GetLocalVIsual)))) "/Game/Objects/Plants/BP_PlantVisual_Parent.BP_PlantVisual_Parent_C" :!class /Script/Engine.PrimitiveComponent)
      (Utilities|IsValid _array_element
        (:Is%20Valid
          (bind _asbp_plant_visual_parent (Utilities|Casting|CastToBP_PlantVisual_Parent _array_element))
          (if (== (Variables|Default|GetPlantIndex) (Variables|/Game/Objects/Plants/BP_PlantVisual_Parent.BP_PlantVisual_Parent_C|GetPlantIndex _asbp_plant_visual_parent))
            (if (and (< _plantindex 5) (> _plantindex 0))
              (if (>= (Math|Vector|VectorLength (- (Transformation|GetActorLocation _array_element) _returnvalue)) 5e+01)
                (Transformation|SetActorLocation (+ (* (Math|Vector|Normalize (- (Transformation|GetActorLocation _array_element) _returnvalue)) (* (Utilities|Time|GetWorldDeltaSeconds) (Variables|Default|GetFusionSpeed))) _returnvalue) false false)
                (else
                  (Variables|Default|SetCouplePlant _asbp_plant_visual_parent)
                  (Game|SpawnActorfromClass "/Game/Objects/BP_Seed.BP_Seed_C" (Math|Transform|MakeTransform (+ (Math|Vector|Lerp(Vector) (Transformation|GetActorLocation _array_element) _returnvalue 0.5) "0, 0,100.000000") (Transformation|GetWorldRotation (Variables|Default|GetSpawnSeedDirection)) "1,1,1") "Undefined" 0 false (Utilities|Select :Index (Variables|Default|GetPlantIndex) :Option%200 0 :Option%201 2 :Option%202 3 :Option%203 4 :Option%204 5) true 0)
                  (Game|SpawnActorfromClass "/Game/Sounds/BP_SFXPlantFusion.BP_SFXPlantFusion_C" (Math|Conversions|ToTransform(Vector) (Math|Vector|Lerp(Vector) (Transformation|GetActorLocation _array_element) _returnvalue 0.5)) "Undefined" 0 0)
                  (bind _output_get (Variables|Default|SetMasterPlantTemp (Variables|/Game/Objects/Plants/BP_PlantVisual_Parent.BP_PlantVisual_Parent_C|GetMaster _asbp_plant_visual_parent)))
                  (Actor|DestroyActor (Variables|Default|GetVisuals))
                  (Actor|DestroyActor (Variables|BP_Plant_C|GetVisuals (Variables|/Game/Objects/Plants/BP_PlantVisual_Parent.BP_PlantVisual_Parent_C|GetMaster _asbp_plant_visual_parent)))
                  (Actor|DestroyActor _output_get)
                  (Actor|DestroyActor))))
            (else
              ;[1 1 1] Degen
              (if (< (/ (Transformation|GetDistanceTo _asbp_plant_visual_parent) 5e+01) (Variables|/Game/Objects/Plants/BP_PlantVisual_Parent.BP_PlantVisual_Parent_C|GetSphereScale _asbp_plant_visual_parent))
                (Variables|Default|SetLifeRemaining (- (Variables|Default|GetLifeRemaining) (* (Variables|/Game/Objects/Plants/BP_PlantVisual_Parent.BP_PlantVisual_Parent_C|GetAreaDegenValue _asbp_plant_visual_parent) (Utilities|Time|GetWorldDeltaSeconds))))))))))))

(fn WateringPlant
  (for _array_element (Variables|Default|GetVisuals)
    (Variables|Default|SetBP_PlantVisualParent _array_element)
    (switch int (Variables|Water|GetNumberOfDick)
      (:1
        (CallFunction|DickSray (Variables|Default|GetArrow1)))
      (:2
        (CallFunction|DickSray (Variables|Default|GetArrow1))
        (CallFunction|DickSray (Variables|Default|GetArrow2)))
      (:3
        (CallFunction|DickSray (Variables|Default|GetArrow1))
        (CallFunction|DickSray (Variables|Default|GetArrow2))
        (CallFunction|DickSray (Variables|Default|GetArrow3))))))

(fn Weed
  (bind _returnvalue (Math|Random|RandomFloatinRange 0.0 3.6e+02))
  (bind _arearadius (Variables|Default|GetAreaRadius))
  (bind _returnvalue_2 (* 5e+01 _arearadius))
  (bind _returnvalue_3 (* _returnvalue_2 1.5))
  (bind _returnvalue_4 (* _returnvalue_2 2.5))
  (bind _returnvalue_5 (Math|Random|RandomFloatinRange _returnvalue_3 _returnvalue_4))
  (bind _returnvalue_6 (CallFunction|ProbabilityPerSecond (Variables|Default|GetWeedRate)))
  (if _returnvalue_6
    (Game|SpawnActorfromClass "/Game/Objects/Plants/BP_Plant_ChildA.BP_Plant_ChildA_C" (Math|Transform|MakeTransform (+ (Transformation|GetActorLocation) (Math|Vector|MakeVector (* _returnvalue_5 (Math|Trig|Cos(Degrees) _returnvalue)) (* _returnvalue_5 (Math|Trig|Sin(Degrees) _returnvalue)) 0.0)) "0, 0, 0" "1,1,1") "Undefined" 0 true 0)))

(fn ProbabilityPerSecond
  (params (Rate :type Float%20%28single-precision%29))
  (return (< (Math|Random|RandomFloatinRange 0.0 1.0) (* Rate (Utilities|Time|GetWorldDeltaSeconds)))))

(fn BudGrowing
  (bind _output_get (Variables|Default|SetSeedSpawnTimerCurrent (- (Variables|Default|GetSeedSpawnTimerCurrent) (Utilities|Time|GetWorldDeltaSeconds))))
  (if (<= _output_get 0.0)
    (CallFunction|SpawnSeed)
    (Bud|InitSpawnSeedTimer)))

(fn InitSpawnSeedTimer
  (Variables|Default|SetSeedSpawnTimerCurrent (Variables|Default|GetSeedSpawnTimeMax)))

(fn BudUpdateScaleValue
  (Variables|Bud|SetBudScale (+ 0.1 (* (- 1.0 (/ (Variables|Default|GetSeedSpawnTimerCurrent) (Variables|Default|GetSeedSpawnTimeMax))) 0.5))))

(fn BudFeed
  (Variables|Default|SetSeedSpawnTimerCurrent (- (Variables|Default|GetSeedSpawnTimerCurrent) (Variables|Bud|GetBudWaterTimeBonus))))

(fn DickSray
  (params (Dick :type Scene%20Component%20Object%20Reference))
  (bind _returnvalue (Transformation|GetWorldTransform Dick))
  (bind _bp_plantvisualparent (Variables|Default|GetBP_PlantVisualParent))
  (bind _defaultsceneroot (Variables|/Game/Objects/Plants/BP_PlantVisual_Parent.BP_PlantVisual_Parent_C|GetDefaultSceneRoot _bp_plantvisualparent))
  (bind _returnvalue_2 (Transformation|GetWorldLocation _defaultsceneroot))
  (bind _returnvalue_3 (Game|SpawnActorfromClass "/Game/Objects/BP_DropOfPiss.BP_DropOfPiss_C" (Math|Transform|MakeTransform (Math|Vector|MakeVector (.x _returnvalue_2) (.y _returnvalue_2) (.z (.location _returnvalue))) (Math|Rotator|CombineRotators (.rotation _returnvalue) (Math|Rotator|MakeRotator (Math|Random|RandomFloatinRange -0.2 0.2) (Math|Random|RandomFloatinRange -0.2 0.2) (Math|Random|RandomFloatinRange -0.2 0.2))) "1,1,1") "Undefined" 0 _bp_plantvisualparent self true 0))
  (Variables|/Game/Objects/BP_DropOfPiss.BP_DropOfPiss_C|SetSpeed _returnvalue_3 7e+02))

(fn ReplicatePlant
  (bind _returnvalue (Transformation|GetActorLocation))
  (bind _tilesize (Variables|Default|GetTileSize))
  (bind _returnvalue_2 (* _tilesize 1e+02))
  (bind (_x _y) (Utilities|ForEachReplication (Variables|Default|GetDisplayDistance))
    (:LoopBody
      (bind _returnvalue_3 (Game|SpawnActorfromClass (Utilities|Select :Index (Variables|Default|GetPlantIndex) :Option%200 "/Game/Objects/Plants/BP_PlantVisual_Child0.BP_PlantVisual_Child0_C" :Option%201 "/Game/Objects/Plants/BP_PlantVisual_Child1.BP_PlantVisual_Child1_C" :Option%202 "/Game/Objects/Plants/BP_PlantVisual_Child2.BP_PlantVisual_Child2_C" :Option%203 "/Game/Objects/Plants/BP_PlantVisual_Child3.BP_PlantVisual_Child3_C" :Option%204 "/Game/Objects/Plants/BP_PlantVisual_Child4.BP_PlantVisual_Child4_C" :Option%205 "/Game/Objects/Plants/BP_PlantVisual_Child5.BP_PlantVisual_Child5_C") (Math|Transform|MakeTransform (Math|Vector|MakeVector (+ (* _x _returnvalue_2) (.x _returnvalue)) (+ (* _y _returnvalue_2) (.y _returnvalue)) 0.0) "0, 0, 0" (Math|Vector|MakeVector 1.0 1.0 1.0)) "Undefined" 0 0))
      (bind _asbp_plant_visual_parent (Utilities|Casting|CastToBP_PlantVisual_Parent _returnvalue_3))
      (Variables|/Game/Objects/Plants/BP_PlantVisual_Parent.BP_PlantVisual_Parent_C|SetSphereScale _asbp_plant_visual_parent (Variables|Default|GetAreaRadius))
      (Variables|/Game/Objects/Plants/BP_PlantVisual_Parent.BP_PlantVisual_Parent_C|SetOffsest _asbp_plant_visual_parent (Math|Vector2D|MakeVector2D (* _x _returnvalue_2) (* _y _returnvalue_2)))
      (Variables|/Game/Objects/Plants/BP_PlantVisual_Parent.BP_PlantVisual_Parent_C|SetPlantIndex _asbp_plant_visual_parent (Variables|Default|GetPlantIndex))
      (Variables|/Game/Objects/Plants/BP_PlantVisual_Parent.BP_PlantVisual_Parent_C|SetAreaDegenValue _asbp_plant_visual_parent (Variables|Default|GetAgressivity))
      (Variables|/Game/Objects/Plants/BP_PlantVisual_Parent.BP_PlantVisual_Parent_C|SetMaster _asbp_plant_visual_parent self)
      (Utilities|Array|Add (Variables|Default|GetVisuals) _asbp_plant_visual_parent)
      (if (and (== _x 0) (== _y 0))
        (Variables|Default|SetLocalVIsual _returnvalue_3)))))

(fn LifeGain
  (Variables|Default|SetPreviousLife (Variables|Default|GetCurrentLife))
  (bind _output_get (Variables|Default|SetCurrentLife (Variables|Default|GetLifeRemaining)))
  (return (/ (- _output_get (Variables|Default|GetPreviousLife)) (Variables|Default|GetLifeMax))))

(fn SetValues
  (params (LifeMax :type Float%20%28single-precision%29) (SeedSpawnTimeMax :type Float%20%28single-precision%29) (FusionSpeed :type Float%20%28single-precision%29) (PlantIndex :type Integer) (Agressivity :type Float%20%28single-precision%29) (AreaRadius :type Float%20%28single-precision%29) (WeedRate :type Float%20%28single-precision%29) (IsWateringPlant :type Boolean) (WaterAddTime :type Float%20%28single-precision%29) (BudWaterTimeBonus :type Float%20%28single-precision%29) (IsPissBooster :type Boolean))
  (Variables|Default|SetLifeMax LifeMax)
  (Variables|Default|SetSeedSpawnTimeMax SeedSpawnTimeMax)
  (Variables|Default|SetFusionSpeed FusionSpeed)
  (Variables|Default|SetPlantIndex PlantIndex)
  (Variables|Default|SetAgressivity Agressivity)
  (Variables|Default|SetAreaRadius AreaRadius)
  (Variables|Default|SetWeedRate WeedRate)
  (Variables|Default|SetIsWateringPlant IsWateringPlant)
  (Variables|Default|SetWaterAddTime WaterAddTime)
  (Variables|Bud|SetBudWaterTimeBonus BudWaterTimeBonus)
  (Variables|Default|SetIsPissBooster IsPissBooster))