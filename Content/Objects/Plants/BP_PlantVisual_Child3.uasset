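; BP_PlantVisual_Child3 is a plant visual variant that adds an animated wind turbine, built on a parent Blueprint.
; On BeginPlay it registers the area visual, skeletal mesh and turbine in AllMeshes before running the parent logic.
; Each tick it runs the parent tick, spins the turbine anchor around yaw at a constant frame-rate-independent speed, and moves the point light to the Scene component's world location.
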(event EventBeginPlay
  (Variables|Default|SetAllMeshes (Utilities|Array|MakeArray (Variables|Default|GetPlantAreaVisual) (Variables|Default|GetSkeletalMesh) (Variables|Default|GetWind_Turbine)))
  (|CallParentFunction)
  (Utilities|FlowControl|Delay 0.2))

(event EventTick
  (params (DeltaSeconds :type Float%20%28single-precision%29))
  (|CallParentFunction DeltaSeconds)
  (Transformation|AddRelativeRotation (Variables|Default|GetAnchorWindTurbine) (Math|Rotator|MakeRotator 0.0 0.0 (* DeltaSeconds 6e+01)) false false)
  ;[1 1 1] set light loc
  (Transformation|SetWorldLocation (Variables|Default|GetPointLight) (Transformation|GetWorldLocation (Variables|Default|GetScene)) false false))

(fn ConstructionScript
  (|CallParentFunction))