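; BP_Plant_Child3 is a plant variant that alters the level's height fog when it begins play.
; On BeginPlay it runs the parent logic, then a timeline drives the density and start distance of the first ExponentialHeightFog actor found.
; The construction script sets plant index 3, stretches AnchorScaleTemp to double height, and passes this variant's lifespan, seeding, fusion, aggressivity, area and watering tuning to SetValues.
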(event EventBeginPlay
  (|CallParentFunction)
  (bind _outactors (Actor|GetAllActorsOfClass "/Script/Engine.ExponentialHeightFog"))
  (bind (_direction _newtrack_0 _dist) (Timeline|Timeline_0 Play)
    (:Update
      (Class|ExponentialHeightFogComponent|SetFogDensity (Variables|/Script/Engine.ExponentialHeightFog|GetComponent (Utilities|Array|Get(acopy) _outactors)) _newtrack_0)
      (Class|ExponentialHeightFogComponent|SetStartDistance (Variables|/Script/Engine.ExponentialHeightFog|GetComponent (Utilities|Array|Get(acopy) _outactors)) _dist))))

(event Collision|EventActorBeginOverlap
  (params (OtherActor :type Actor%20Object%20Reference)))

(event EventTick
  (params (DeltaSeconds :type Float%20%28single-precision%29))
  (|CallParentFunction DeltaSeconds))

(fn ConstructionScript
  (|CallParentFunction)
  (Variables|Default|SetPlantIndex 3)
  (Transformation|SetRelativeScale3D (Variables|Default|GetAnchorScaleTemp) "1.000000,1.000000,2.000000")
  (CallFunction|SetValues 1.2e+02 5e+02 7.5 3 1.0 4.0 0.1 false 0.4 0.8 false))