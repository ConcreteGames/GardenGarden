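; Piss droplet projectile, from a plant or the hero, that waters plants and pushes seeds on impact.
; It moves forward each tick while pitching down to fake an arc, mirroring its transform to an HISM visual, larger and differently shaded when boosted.
; On first hitting ground it splashes with decal, particles and sound, waters overlapping plants and impulses seeds.
; A seed hit only pushes; both impacts call ReplaceInTile, then destroy the drop.
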(event OnComponentBeginOverlap(PissCollider)
  (params (OverlappedComponent :type Primitive%20Component%20Object%20Reference) (OtherActor :type Actor%20Object%20Reference) (OtherComp :type Primitive%20Component%20Object%20Reference) (OtherBodyIndex :type Integer) (bFromSweep :type Boolean) (SweepResult :type Hit%20Result%20Structure%20%28by%20ref%29))
  ;[1 1 1] Collide the ground
  (Utilities|Casting|CastToBP_Tiling OtherActor
    (:then
      (Utilities|FlowControl|DoOnce false
        (:Completed
          (CallFunction|VFXSplash)
          (bind _isreplaced (CallFunction|ReplaceinTile (Variables|Default|GetPissCollider)))
          (if _isreplaced
            (CallFunction|VFXSplash)
            (CallFunction|SFXSplash))
          (CallFunction|PissonFlourinPlantArea)
          (CallFunction|GetCollidingSeedsAnPushThem)
          (CallFunction|VFXSplash)
          (CallFunction|SFXSplash)
          ;[1 1 1] Death
          (CallFunction|Death))))
    (:CastFailed
      ;[1 1 1] Collide a seed
      (Utilities|Casting|CastToBP_Seed OtherActor)
      (Utilities|FlowControl|DoOnce false
        (:Completed
          (CallFunction|ReplaceinTile (Variables|Default|GetPissCollider))
          (CallFunction|GetCollidingSeedsAnPushThem)
          ;[1 1 1] Death
          (CallFunction|Death))))))

(event EventBeginPlay
  (bind _arrow (Variables|Default|GetArrow))
  (bind _hism_visual (Variables|Default|GetHISM_Visual))
  ;[1 0.925 0] BEGIN PLAY
  (|CallParentFunction)
  (CallFunction|HISMSetSMandMat _hism_visual)
  (CallFunction|SpawnVisualandReplications _hism_visual (select (Variables|Default|GetIsBoosted) "0.800000,0.800000,0.800000" "0.400000,0.400000,0.400000"))
  ;[1 1 1] Comment
  (Transformation|SetActorRotation (Transformation|GetWorldRotation _arrow))
  (Transformation|SetWorldRotation _arrow "0, 0, 0" false false)
  (Transformation|AddRelativeRotation (Variables|Default|GetDefaultSceneRoot) (Math|Rotator|MakeRotator (Math|Random|RandomFloatinRange -2.0 2.0) (Math|Random|RandomFloatinRange -2.0 2.0) (Math|Random|RandomFloatinRange -2.0 2.0)) false false))

(event EventTick
  (params (DeltaSeconds :type Float%20%28single-precision%29))
  (bind _returnvalue (Utilities|Time|GetWorldDeltaSeconds))
  (bind _pisscollider (Variables|Default|GetPissCollider))
  (bind _returnvalue_2 (Transformation|GetWorldRotation _pisscollider))
  (bind _returnvalue_3 (* _returnvalue 1.5e+02))
  (bind _returnvalue_4 (- (.pitch _returnvalue_2) _returnvalue_3))
  ;[0 1 0.1034] EVENT TICK
  (CallFunction|UpdateHISMTransform (Variables|Default|GetHISM_Visual) (Variables|Default|GetVisual))
  (Transformation|AddLocalOffset _pisscollider (Math|Vector|MakeVector (* DeltaSeconds (select (Utilities|IsValid (Variables|Default|GetPlantMaster)) (Variables|Default|GetSpeed) (Variables|/Game/Character/BP_HeroN.BP_HeroN_C|GetPissSpeed (.AsBP%20Hero%20N (Utilities|Casting|CastToBP_HeroN (Game|Player|GetPlayerPawn 0)))))) 0.0 0.0) false false)
  (Transformation|SetWorldRotation _pisscollider (Math|Rotator|MakeRotator (.roll _returnvalue_2) (select (<= _returnvalue_4 -9e+01) -9e+01 _returnvalue_4) (.yaw _returnvalue_2)) false false))

(fn ConstructionScript
  (|CallParentFunction))

(fn VFXSplash
  (bind _pisscollider (Variables|Default|GetPissCollider))
  (bind _returnvalue (Transformation|GetWorldLocation _pisscollider))
  (Utilities|FlowControl|Sequence
    (:then_0
      (Rendering|Decal|SpawnDecalatLocation "/Game/Objects/Piss/M_Piss2.M_Piss2" "60.000000,30.000000,30.000000" (Math|Vector|MakeVector (.x _returnvalue) (.y _returnvalue) 0.0) (Math|Rotator|MakeRotator 0.0 -9e+01 (Math|Random|RandomFloatinRange 0.0 3.6e+02)) 5.0))
    (:then_1
      (Effects|SpawnEmitteratLocation "/Game/Objects/Piss/PS_Splash.PS_Splash" (Math|Vector|MakeVector (.x _returnvalue) (.y _returnvalue) 0.0)))))

(fn PissonFlourinPlantArea
  ;[1 1 1] if collide a PlantArea
  (for _array_element (Collision|GetOverlappingActors (Variables|Default|GetPissCollider) "/Game/Objects/Plants/BP_PlantVisual_Parent.BP_PlantVisual_Parent_C" :!class /Script/Engine.PrimitiveComponent)
    ;[1 1 1] Water this plant
    (bind _asbp_plant_visual_parent (Utilities|Casting|CastToBP_PlantVisual_Parent _array_element))
    (Utilities|IsValid (Variables|/Game/Objects/Plants/BP_PlantVisual_Parent.BP_PlantVisual_Parent_C|GetMaster _asbp_plant_visual_parent)
      (:Is%20Valid
        (Default|Water (Variables|/Game/Objects/Plants/BP_PlantVisual_Parent.BP_PlantVisual_Parent_C|GetMaster _asbp_plant_visual_parent))))))

(fn Death
  (Actor|SetLifeSpan 0.01)
  (Collision|SetCollisionEnabled (Variables|Default|GetPissCollider) "NoCollision"))

(fn SFXSplash
  (Game|SpawnActorfromClass "/Game/Sounds/BP_SFXSoundSquirt.BP_SFXSoundSquirt_C" (Math|Transform|MakeTransform (Transformation|GetWorldLocation (Variables|Default|GetPissCollider)) "0, 0, 0" "1,1,1") "Undefined" 0 0))

(fn PushSeed
  (params (Seed :type BP%20Seed%20Object%20Reference))
  (Physics|AddImpulse (Variables|/Game/Objects/BP_Seed.BP_Seed_C|GetSeedCollider Seed) (* (Math|Rotator|GetRotationXVector (Transformation|GetWorldRotation (Variables|Default|GetPissCollider))) 4e+03) "None" false))

(fn GetCollidingSeedsAnPushThem
  (for _array_element (Collision|GetOverlappingActors (Variables|Default|GetPissCollider) "/Game/Objects/BP_Seed.BP_Seed_C" :!class /Script/Engine.PrimitiveComponent)
    (bind _asbp_seed (Utilities|Casting|CastToBP_Seed _array_element))
    (CallFunction|PushSeed _asbp_seed)))

(fn HISMSetSMandMat
  (params (HISM :type Static%20Mesh%20Component%20Object%20Reference))
  (Components|StaticMesh|SetStaticMesh HISM "/Game/Objects/Piss/SM_Piss.SM_Piss")
  (Rendering|Material|SetMaterial HISM 0 (select (Variables|Default|GetIsBoosted) "/Game/Objects/Piss/M_PissBoosted.M_PissBoosted" "/Game/Objects/Piss/M_Piss.M_Piss")))