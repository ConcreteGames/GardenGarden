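; BP_Jet is the piss jet, a particle stream switched on and off by events, that waters plants and pushes seeds.
; Each particle collision moves DropCollider to the hit point, makes overlapped plants' masters Drink and applies a forward impulse to overlapped seeds.
; Splash sound and normal or boosted emitters are gated by camera distance, with emitters also requiring on-screen visibility.
; A short timeline, restarted on each splash, stops the looping sound once impacts cease.
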(event OnParticleCollide(PS_Jet)
  (params (EventName :type Name :default "None") (EmitterTime :type Float%20%28single-precision%29) (ParticleTime :type Integer) (Location :type Vector :default "0, 0, 0") (Velocity :type Vector :default "0, 0, 0") (Direction :type Vector :default "0, 0, 0") (Normal :type Vector :default "0, 0, 0") (BoneName :type Name :default "None") (PhysMat :type Physical%20Material%20Object%20Reference))
  (CallFunction|PissVFXandSFX Location)
  (Transformation|SetWorldLocation (Variables|Default|GetDropCollider) Location false false)
  (CallFunction|WetFloorinPlantArea)
  (CallFunction|PushSeed))

(event Custom|ActivateJet
  (Components|Activation|Activate (Variables|Default|GetPS_Jet) false))

(event Custom|SFX_Splash
  (bind _a_pisssound (Variables|Default|GetA_PissSound))
  (bind _returnvalue (Class|FMODAudioComponent|IsPlaying _a_pisssound))
  (if _returnvalue
    (Timeline|SFXSplashDuration PlayFromStart
      (:Finished
        (Class|FMODAudioComponent|Stop (Variables|Default|GetA_PissSound))))
    (else
      (Class|FMODAudioComponent|Play _a_pisssound)
      (Timeline|SFXSplashDuration PlayFromStart))))

(event Custom|DesactivateJet
  (Components|Activation|Deactivate (Variables|Default|GetPS_Jet)))

(event EventBeginPlay
  ;[0.04042 1 0] BEGIN PLAY
  (Components|Timeline|SetTimelineLength (Variables|Default|GetSFXSplashDuration) 0.2))

(fn ConstructionScript)

(fn PissVFXandSFX
  (params (InputPin :type Vector))
  (bind _dropcollider (Variables|Default|GetDropCollider))
  (Utilities|FlowControl|Sequence
    (:then_0
      (if (CallFunction|IsClosertoCameraThan (Variables|Default|GetDropCollider) 1.5e+03)
        (CallFunction|SFXSplash)))
    (:then_1
      (if (and (CallFunction|IsonScreen _dropcollider) (CallFunction|IsClosertoCameraThan _dropcollider 2.2e+03))
        (if (Variables|Default|GetIsBoosted)
          (Effects|SpawnEmitteratLocation "/Game/Objects/Piss/PS_SplashBoosted.PS_SplashBoosted" InputPin)
          (else
            (Effects|SpawnEmitteratLocation "/Game/Objects/Piss/PS_Splash.PS_Splash" InputPin)))))))

(fn WetFloorinPlantArea
  ;[1 1 1] if collide a PlantArea
  (for _array_element (Collision|GetOverlappingActors (Variables|Default|GetDropCollider) "/Game/Objects/Plants/BP_PlantVisual_Parent.BP_PlantVisual_Parent_C" :!class /Script/Engine.PrimitiveComponent)
    ;[1 1 1] Water this plant
    (bind _asbp_plant_visual_parent (Utilities|Casting|CastToBP_PlantVisual_Parent _array_element))
    (Utilities|IsValid (Variables|/Game/Objects/Plants/BP_PlantVisual_Parent.BP_PlantVisual_Parent_C|GetMaster _asbp_plant_visual_parent)
      (:Is%20Valid
        (Default|Drink (Variables|/Game/Objects/Plants/BP_PlantVisual_Parent.BP_PlantVisual_Parent_C|GetMaster _asbp_plant_visual_parent))))))

(fn PushSeed
  (for _array_element (Collision|GetOverlappingActors (Variables|Default|GetDropCollider) "/Game/Objects/Seed/BP_Seed.BP_Seed_C" :!class /Script/Engine.PrimitiveComponent)
    (bind _asbp_seed (Utilities|Casting|CastToBP_Seed _array_element))
    (Physics|AddImpulse (Variables|/Game/Objects/Seed/BP_Seed.BP_Seed_C|GetSeedCollider _asbp_seed) (* (Math|Rotator|GetRotationXVector (Transformation|GetWorldRotation (Variables|Default|GetDropCollider))) (Variables|Default|GetSeedImpulseForce)) "None" false)))