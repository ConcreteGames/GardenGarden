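; A piss droplet projectile that waters plants, shoves seeds and splashes on impact.
; Each tick its collider moves forward and pitches down into an arc, using its own speed with a valid PlantMaster or the hero's PissSpeed otherwise, then calls ReplaceInTile.
; The first overlap outside its plant owner or master expires it, plays a squirt sound near the player, and on tiling leaves a random decal or particle burst.
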(event OnComponentBeginOverlap(Coll)
  (params (OverlappedComponent :type Primitive%20Component%20Object%20Reference) (OtherActor :type Actor%20Object%20Reference) (OtherComp :type Primitive%20Component%20Object%20Reference) (OtherBodyIndex :type Integer) (bFromSweep :type Boolean) (SweepResult :type Hit%20Result%20Structure%20%28by%20ref%29))
  (if (not (or (== OtherActor (Variables|Default|GetPlantOwner)) (== OtherActor (Variables|Default|GetPlantMaster))))
    (Variables|Default|SetOtherActor OtherActor)
    (Utilities|FlowControl|DoOnce false
      (:Completed
        (Actor|SetLifeSpan 0.03)
        (Utilities|FlowControl|Sequence
          (:then_0
            (if (< (Math|Vector|VectorLength (- (Transformation|GetWorldLocation (Variables|Default|GetColl)) (.location (Transformation|GetActorTransform (Game|Player|GetPlayerPawn 0))))) 1e+03)
              (Game|SpawnActorfromClass "/Game/Sounds/BP_SFXSoundSquirt.BP_SFXSoundSquirt_C" (Math|Transform|MakeTransform (Transformation|GetWorldLocation (Variables|Default|GetColl)) "0, 0, 0" "1,1,1") "Undefined" 0 0))
            ;[1 1 1] Water plant
            (bind _asbp_plant (Utilities|Casting|CastToBP_Plant (Variables|Default|GetOtherActor))
              (:then
                (Default|Water _asbp_plant))
              (:CastFailed
                ;[1 1 1] Push sheed by pissing on it
                (bind _asbp_seed (Utilities|Casting|CastToBP_Seed (Variables|Default|GetOtherActor)))
                (Physics|AddImpulse (Variables|/Game/Objects/BP_Seed.BP_Seed_C|GetSeedCollider _asbp_seed) (* (Math|Rotator|GetRotationXVector (Transformation|GetWorldRotation (Variables|Default|GetColl))) 4e+03) "None" false))))
          (:then_1
            (Utilities|Casting|CastToBP_TilingClass (Utilities|GetClass (Variables|Default|GetOtherActor)))
            (CallFunction|Squirt)))))))

(event EventBeginPlay
  (bind _arrow (Variables|Default|GetArrow))
  ;[1 0.925 0] BEGIN PLAY
  ;[1 1 1] Comment
  (Transformation|SetActorRotation (Transformation|GetWorldRotation _arrow))
  (Transformation|SetWorldRotation _arrow "0, 0, 0" false false)
  (Transformation|AddRelativeRotation (Variables|Default|GetDefaultSceneRoot) (Math|Rotator|MakeRotator (Math|Random|RandomFloatinRange -2.0 2.0) (Math|Random|RandomFloatinRange -2.0 2.0) (Math|Random|RandomFloatinRange -2.0 2.0)) false false))

(event EventTick
  (params (DeltaSeconds :type Float%20%28single-precision%29))
  (bind _returnvalue (Utilities|Time|GetWorldDeltaSeconds))
  (bind _coll (Variables|Default|GetColl))
  (bind _returnvalue_2 (Transformation|GetWorldRotation _coll))
  (bind _returnvalue_3 (* _returnvalue 1.5e+02))
  (bind _returnvalue_4 (- (.pitch _returnvalue_2) _returnvalue_3))
  ;[0 1 0.1034] EVENT TICK
  (Transformation|AddLocalOffset _coll (Math|Vector|MakeVector (* DeltaSeconds (select (Utilities|IsValid (Variables|Default|GetPlantMaster)) (Variables|Default|GetSpeed) (Variables|/Game/Character/BP_HeroN.BP_HeroN_C|GetPissSpeed (.AsBP%20Hero%20N (Utilities|Casting|CastToBP_HeroN (Game|Player|GetPlayerPawn 0)))))) 0.0 0.0) false false)
  (Transformation|SetWorldRotation _coll (Math|Rotator|MakeRotator (.roll _returnvalue_2) (select (<= _returnvalue_4 -9e+01) -9e+01 _returnvalue_4) (.yaw _returnvalue_2)) false false)
  (CallFunction|ReplaceinTile (Variables|Default|GetColl)))

(fn ConstructionScript
  (|CallParentFunction))

(fn Squirt
  (bind _coll (Variables|Default|GetColl))
  (bind _returnvalue (Transformation|GetWorldLocation _coll))
  (if (Math|Random|RandomBool)
    (Rendering|Decal|SpawnDecalatLocation "/Game/Objects/Piss/M_Piss2.M_Piss2" "60.000000,30.000000,30.000000" _returnvalue (Math|Rotator|MakeRotator 0.0 -9e+01 (Math|Random|RandomFloatinRange 0.0 3.6e+02)) 5.0)
    (else
      (Effects|SpawnEmitteratLocation "/Game/Objects/Piss/PS_Piss.PS_Piss" _returnvalue))))