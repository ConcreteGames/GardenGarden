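; Parent Blueprint for world objects that copies itself across a tiled grid around its position.
; BeginPlay caches TileSize and DisplayDistance from the first BP_Tiling actor for use by Replicate.
; Replicate loops over the grid cells within DisplayDistance, skipping the center, and spawns its own class at tile-sized XY offsets.
; Copies spawn with IsActive false and are stored in Tiles; Replicate is not called within this Blueprint.
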(event EventBeginPlay
  ;[1 1 1] Get TileSize & DisplayDistance for Replicate function
  (bind _outactors (Actor|GetAllActorsOfClass "/Game/Levels/Tiling/BP_Tiling.BP_Tiling_C"))
  (Variables|Default|SetTileSize (Variables|/Game/Levels/Tiling/BP_Tiling.BP_Tiling_C|GetTileSize (Utilities|Array|Get(acopy) _outactors)))
  (Variables|Default|SetDisplayDistance (Variables|/Game/Levels/Tiling/BP_Tiling.BP_Tiling_C|GetDisplayDistance (Utilities|Array|Get(acopy) _outactors))))

(fn ConstructionScript)

(fn Replicate
  (bind _returnvalue (Transformation|GetActorLocation))
  (bind _tilesize (Variables|Default|GetTileSize))
  (bind _returnvalue_2 (* _tilesize 1e+02))
  (bind (_x _y) (Utilities|ForEachReplication (Variables|Default|GetDisplayDistance))
    (:LoopBody
      (if (not (and (== _x 0) (== _y 0)))
        (bind _returnvalue_3 (Game|SpawnActorfromClass (Utilities|GetClass self) (Math|Transform|MakeTransform (Math|Vector|MakeVector (+ (* _x _returnvalue_2) (.x _returnvalue)) (+ (* _y _returnvalue_2) (.y _returnvalue)) 0.0) "0, 0, 0" (Math|Vector|MakeVector 1.0 1.0 1.0)) "Undefined" 0 false 0))
        (Utilities|Array|Add (Variables|Default|GetTiles) _returnvalue_3)))))