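; Physics seed actor that pops up with random spin, can be grabbed and thrown, and turns into a plant matching its Index.
; Tick runs a state machine (air, ground, hand, throw), pinning the held seed to the hand anchor.
; A floor overlap while thrown spawns BP_Plant facing the hero's rotation and destroys the seed.
; A looping downward trace launches seeds with no floor beneath back toward world origin.
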(event OnComponentBeginOverlap(TriggerFloor)
  (params (OverlappedComponent :type Primitive%20Component%20Object%20Reference) (OtherActor :type Actor%20Object%20Reference) (OtherComp :type Primitive%20Component%20Object%20Reference) (OtherBodyIndex :type Integer) (bFromSweep :type Boolean) (SweepResult :type Hit%20Result%20Structure%20%28by%20ref%29))
  ;[1 1 1] SFX Fall in grass
  (Audio|Components|Audio|Play (Variables|Default|GetFallGrass) 0.0)
  (if (Utilities|Enum|Equal(Enum) (Variables|Default|GetState) "NewEnumerator4")
    (CallFunction|SpawnPlant)
    (Actor|DestroyActor)))

(event Custom|SeedGrabed
  (params (HandAnchor :type Scene%20Component%20Object%20Reference))
  (bind _seedcollider (Variables|Default|GetSeedCollider))
  (Variables|Default|SetTempHand HandAnchor)
  ;[1 1 1] DIsable phys & gravity
  (Physics|SetSimulatePhysics _seedcollider false)
  (Physics|SetEnableGravity _seedcollider false)
  (Variables|Default|SetState "NewEnumerator1"))

(event Custom|TestFloor
  (bind _seedcollider (Variables|Default|GetSeedCollider))
  (bind _seedcollider_2 (Variables|Default|GetSeedCollider))
  (bind _returnvalue (Transformation|GetWorldLocation _seedcollider_2))
  (bind _returnvalue_2 (Transformation|GetWorldLocation _seedcollider))
  (bind _returnvalue_3 (- "0, 0, 0" _returnvalue))
  (bind _returnvalue_4 (Math|Vector|MakeVector (.x _returnvalue_3) (.y _returnvalue_3) 0.0))
  (bind _returnvalue_5 (Math|Vector|Normalize _returnvalue_4))
  (bind _returnvalue_6 (* _returnvalue_5 5e+02))
  (if (not (Variables|Default|GetImpulseBack))
    (bind _returnvalue_7 (Collision|LineTraceForObjects _returnvalue_2 (+ _returnvalue_2 "0, 0,-10000.000000") (Utilities|Array|MakeArray "ObjectTypeQuery11") false 0 "None"))
    (if (not _returnvalue_7)
      (bind _returnvalue_8 (Physics|GetPhysicsLinearVelocity _seedcollider_2 "None"))
      (Physics|SetPhysicsLinearVelocity _seedcollider_2 (Math|Vector|MakeVector (.x _returnvalue_6) (.y _returnvalue_6) (+ (Math|Float|Absolute(Float) (.Z (Math|Vector|BreakVector _returnvalue_8))) 5e+02)) false "None")
      (Audio|Components|Audio|Play (Variables|Default|GetSFX_woosh_Cue) 0.0)
      (Variables|Default|SetImpulseBack true)
      (Utilities|FlowControl|Delay 0.2)
      (Variables|Default|SetImpulseBack false))))

(event EventBeginPlay
  (bind _seedcollider (Variables|Default|GetSeedCollider))
  ;[1 0.8366 0] BEGIN PLAY
  (|CallParentFunction)
  ;[1 1 1] jump at start
  (Physics|AddImpulse _seedcollider (* (Math|Vector|GetUpVector (Transformation|GetWorldRotation _seedcollider)) (* (Physics|GetMass _seedcollider) 8e+02)) "None" false)
  ;[1 1 1] Add rotation
  (Class|PrimitiveComponent|AddTorqueinDegrees _seedcollider (* (Math|Random|RandomUnitVector) (* (Math|Random|RandomFloatinRange 1.0 5e+01) 1e+03)) "None" true)
  (CallFunction|InitAutoPlantingTimer)
  (CallFunction|SFXPopfromPlant)
  (Utilities|Time|SetTimerbyEvent (delegate Custom|TestFloor) 0.1 true))

(event EventTick
  (params (DeltaSeconds :type Float%20%28single-precision%29))
  (bind _seedcollider (Variables|Default|GetSeedCollider))
  ;[0.09175 1 0] EVENT TICK
  (if (not (Variables|Default|GetIsPlant)) ; If not already plant
    (switch Utilities|FlowControl|Switch|SwitchonE_SeedStates (Variables|Default|GetState)
      (:NewEnumerator0
        (Utilities|TestVelocity
          (:Stop
            (Variables|Default|SetState "NewEnumerator3"))))
      (:NewEnumerator3
        (Utilities|TestVelocity
          (:Moving
            (CallFunction|InitAutoPlantingTimer)
            (if (Variables|Default|GetHasBeenGrabedAtLeastOnce)
              (Variables|Default|SetState "NewEnumerator4")
              (else
                (Variables|Default|SetState "NewEnumerator0"))))))
      (:NewEnumerator1
        (CallFunction|InitAutoPlantingTimer)
        (CallFunction|FixSeedinHand)
        (Variables|Default|SetHasBeenGrabedAtLeastOnce true))
      (:NewEnumerator2
        ;[1 1 1] Enable phys & gravity
        (Physics|SetSimulatePhysics _seedcollider true)
        (Physics|SetEnableGravity _seedcollider true)
        (Variables|Default|SetState "NewEnumerator4")))))

(event EventEndPlay
  (params (EndPlayReason :type EEndPlayReason%20Enum :default "Destroyed"))
  ;[0 0 0] END PLAY
  (Actor|SetLifeSpan (Variables|Default|GetVisualAndReplications) 0.01))

(fn ConstructionScript
  (bind _sm_seed (Variables|Default|GetSM_Seed))
  (|CallParentFunction)
  (CallFunction|LogErer (Utilities|String|ToString(Integer) (Variables|Default|GetIndex)))
  (Rendering|Material|SetMaterial _sm_seed 0 "/Game/Objects/Plants3D/Seed/M_MaterialGraineChapeau.M_MaterialGraineChapeau")
  (CallFunction|LogErer (Utilities|GetDisplayName (Rendering|Material|GetMaterial _sm_seed 0)))
  (Rendering|Material|SetMaterial _sm_seed 1 (Utilities|Select :Index (Variables|Default|GetIndex) :Option%200 0 :Option%201 "/Game/Objects/Plants3D/Seed/M_Graine_1.M_Graine_1" :Option%202 "/Game/Objects/Plants3D/Seed/M_Graine_2.M_Graine_2" :Option%203 "/Game/Objects/Plants3D/Seed/M_Graine_3.M_Graine_3" :Option%204 "/Game/Objects/Plants3D/Seed/M_Graine_4.M_Graine_4" :Option%205 "/Game/Objects/Plants3D/Seed/M_Graine_5.M_Graine_5")))

(fn SpawnPlant
  (bind _seedcollider (Variables|Default|GetSeedCollider))
  (bind _seedcollider_2 (Variables|Default|GetSeedCollider))
  (bind _returnvalue (Transformation|GetWorldTransform _seedcollider_2))
  (bind _returnvalue_2 (Transformation|GetWorldLocation _seedcollider))
  (Variables|Default|SetIsPlant true)
  ;[0.9326 0 1] est-ce bien de faire comme ça ? ça me parraît chelou de créer un BP juste pour un son...
  ;;[1 1 1] SFX Pop
  (Game|SpawnActorfromClass "/Game/Sounds/BP_SFXPlantSpawn.BP_SFXPlantSpawn_C" (Math|Transform|MakeTransform (.location _returnvalue) (.rotation _returnvalue) "1,1,1") "Undefined" 0 0)
  (bind _out_row (CallFunction|GetPlantParam (Variables|Default|GetIndex)))
  (Game|SpawnActorfromClass "/Game/Objects/Plants/BP_Plant.BP_Plant_C" (Math|Transform|MakeTransform (Math|Vector|MakeVector (.x _returnvalue_2) (.y _returnvalue_2) 0.0) (Transformation|GetActorRotation (.AsBP%20Hero%20N (Utilities|Casting|CastToBP_HeroN (Game|Player|GetPlayerPawn 0)))) "1,1,1") "Undefined" 0 _out_row true 0))

(fn InitAutoPlantingTimer
  (Variables|Default|SetAutoPlantingTimerCurrent (Variables|Default|GetAutoPlantingTimer)))

(fn FixSeedinHand
  (bind _temphand (Variables|Default|GetTempHand))
  (bind _returnvalue (Transformation|GetWorldTransform _temphand))
  (Transformation|SetWorldLocationAndRotation (Variables|Default|GetSeedCollider) (.location _returnvalue) (.rotation _returnvalue) false false))

(fn TestifVelocity0
  (bind _returnvalue (Physics|GetPhysicsLinearVelocity (Variables|Default|GetSeedCollider) "None"))
  (return (== (Math|Vector|VectorLength _returnvalue) 0.0)))

(fn UpdateSeedLocation
  (params (HISM :type Hierarchical%20Instanced%20Static%20Mesh%20Component%20Object%20Reference) (SceneAnchor :type Scene%20Component%20Object%20Reference))
  (for _index (range 0 (- (Components|InstancedStaticMesh|GetInstanceCount HISM) 1))
    (Components|InstancedStaticMesh|UpdateInstanceTransform HISM _index (Math|Transform|MakeTransform (+ (Transformation|GetWorldLocation SceneAnchor) (Math|Vector|MakeVector (.x (Utilities|Array|Get(acopy) (Variables|Default|GetVisualsOffsets) _index)) (.y (Utilities|Array|Get(acopy) (Variables|Default|GetVisualsOffsets) _index)) 0.0)) (Transformation|GetWorldRotation SceneAnchor) (.scale (.OutInstanceTransform (Components|InstancedStaticMesh|GetInstanceTransform HISM _index false)))) true false true)))

(fn CircleVisibility
  (Rendering|SetVisibility (Variables|/Game/Objects/BP_SeedVisual.BP_SeedVisual_C|GetCircleSelection (Utilities|Array|Get(acopy) (Variables|Default|GetVisualAndReplications))) false false))

(fn SeedSetSMandMaterial
  (params (HISM :type Hierarchical%20Instanced%20Static%20Mesh%20Component%20Object%20Reference))
  (bind _sm_seed (Variables|Default|GetSM_Seed))
  (CallFunction|LogErer (Utilities|String|ToString(Integer) (Variables|Default|GetIndex)))
  (Rendering|Material|SetMaterial _sm_seed 0 (Utilities|Select :Index (Variables|Default|GetIndex) :Option%200 0 :Option%201 "/Game/Objects/Plants3D/Seed/M_Graine_1.M_Graine_1" :Option%202 "/Game/Objects/Plants3D/Seed/M_Graine_2.M_Graine_2" :Option%203 "/Game/Objects/Plants3D/Seed/M_Graine_3.M_Graine_3" :Option%204 "/Game/Objects/Plants3D/Seed/M_Graine_4.M_Graine_4" :Option%205 "/Game/Objects/Plants3D/Seed/M_Graine_5.M_Graine_5"))
  (CallFunction|LogErer (Utilities|GetDisplayName (Rendering|Material|GetMaterial _sm_seed 0)))
  (Rendering|Material|SetMaterial _sm_seed 0 "/Game/Objects/Plants3D/Seed/M_MaterialGraineChapeau.M_MaterialGraineChapeau"))

(fn SFXPopfromPlant
  (if (not (Variables|Default|GetHasBeenGrabedAtLeastOnce))
    (Audio|Components|Audio|Play (Variables|Default|GetPopSeed) 0.0)))