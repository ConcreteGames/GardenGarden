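; BP_SelectionCircle is a selection marker actor that highlights the seed the player's BP_HeroN has found.
; Each Tick it casts the player character to BP_HeroN and hides itself in game unless SeedFound is true.
; While a valid CurrentSeed is found, it snaps to that seed's SeedCollider and uses a look-at rotation to face the hero's camera like a billboard.
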(event EventTick
  (params (DeltaSeconds :type Float%20%28single-precision%29))
  (bind _asbp_hero_n (Utilities|Casting|CastToBP_HeroN (Game|GetPlayerCharacter 0)))
  (Rendering|SetActorHiddenInGame (not (Variables|/Game/Character/BP_HeroN.BP_HeroN_C|GetSeedFound _asbp_hero_n)))
  (if (Variables|/Game/Character/BP_HeroN.BP_HeroN_C|GetSeedFound _asbp_hero_n)
    (Utilities|IsValid (Variables|/Game/Character/BP_HeroN.BP_HeroN_C|GetCurrentSeed _asbp_hero_n)
      (:Is%20Valid
        (Transformation|SetActorLocationAndRotation (Transformation|GetWorldLocation (Variables|/Game/Objects/BP_Seed.BP_Seed_C|GetSeedCollider (Variables|/Game/Character/BP_HeroN.BP_HeroN_C|GetCurrentSeed _asbp_hero_n))) (Math|Rotator|FindLookatRotation (Transformation|GetActorLocation) (Transformation|GetWorldLocation (Variables|/Game/Character/BP_HeroN.BP_HeroN_C|GetCamera _asbp_hero_n))))))))

(fn ConstructionScript)