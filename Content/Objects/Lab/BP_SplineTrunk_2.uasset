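; Lab actor that grows a winding trunk at runtime from a spline skinned with spline mesh components.
; Tick pushes the last point along its tangent, gradually bends that tangent by AddedRot, then refreshes every mesh segment.
; A looping timeline of short random length adds a point and mesh segment on each finish, occasionally re-rolling the bend.
; Construction script is empty; DrawSpline and random material selection are never run.
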(event EventTick
  (params (DeltaSeconds :type Float%20%28single-precision%29))
  (bind _returnvalue (CallFunction|GetSplineLastPointIndex))
  (bind _returnvalue_2 (CallFunction|GetSplineLastPointIndex))
  (bind _spline (Variables|Default|GetSpline))
  (bind _spline_2 (Variables|Default|GetSpline))
  (bind _returnvalue_3 (Spline|GetTangentatSplinePoint _spline _returnvalue "Local"))
  (bind (_location _tangent) (Spline|GetLocationandTangentatSplinePoint _spline_2 _returnvalue_2 "World"))
  (Spline|SetTangentatSplinePoint _spline _returnvalue (* (Math|Vector|Normalize (Math|Vector|Lerp(Vector) _returnvalue_3 (Math|Vector|RotateVector _returnvalue_3 (Variables|Default|GetAddedRot)) (* 5.0 (Utilities|Time|GetWorldDeltaSeconds)))) (Math|Vector|VectorLength _returnvalue_3)) "Local" false)
  (Spline|SetLocationatSplinePoint _spline_2 _returnvalue_2 (+ _location (* (Math|Vector|Normalize _tangent) (* 5e+02 (Utilities|Time|GetWorldDeltaSeconds)))) "World" true)
  (CallFunction|UpdateSplineVisual))

(event EventBeginPlay
  (bind _returnvalue (CallFunction|GetSplineLastPointIndex))
  (bind _spline (Variables|Default|GetSpline))
  (bind (_location _tangent) (Spline|GetLocationandTangentatSplinePoint _spline _returnvalue "World"))
  (Transformation|SetWorldRotation (Variables|Default|GetTopScene) (Transformation|GetWorldRotation (Variables|Default|GetGrowDirection)) false false)
  (CallFunction|AddMeshSection (- (CallFunction|GetSplineLastPointIndex) 1))
  (Components|Timeline|SetTimelineLength (Variables|Default|GetChangeDirection) (Math|Random|RandomFloatinRange 0.05 0.1) :!label _label)
  (Timeline|ChangeDirection PlayFromStart
    (:Finished
      (Utilities|FlowControl|Sequence
        (:then_0
          (if (Math|Random|RandomBoolwithWeight 0.25)
            (Variables|Default|SetAddedRot (Math|Rotator|MakeRotator 0.0 (select (Math|Random|RandomBool) 45.0 -45.0) (select (Math|Random|RandomBool) 45.0 -45.0))))
          ;[1 1 1] Add point
          (bind _output_get (Variables|Default|SetLastLocation _location))
          (Variables|Default|SetLastTangent _tangent)
          (Spline|AddSplinePoint _spline _output_get "World" true)
          (Spline|SetTangentatSplinePoint _spline (CallFunction|GetSplineLastPointIndex) (Variables|Default|GetLastTangent) "World" true)
          (CallFunction|AddMeshSection (- (CallFunction|GetSplineLastPointIndex) 1)))
        (:then_1
          (goto _label))))))

(fn ConstructionScript)

(fn DrawSpline
  (for _index (range 0 (- (Spline|GetNumberOfSplinePoints (Variables|Default|GetSpline)) 2)) ; On loop autant qu'il y a de débuts\nExemple : 2 points, un seul début, soit first 0 Last 0
    (CallFunction|AddMeshSection _index)))

(fn UpdateSplineVisual
  (bind _spline (Variables|Default|GetSpline))
  (for _index (range 0 (- (Spline|GetNumberOfSplinePoints (Variables|Default|GetSpline)) 2)) ; On loop autant qu'il y a de débuts\nExemple : 2 points, un seul début, soit first 0 Last 0
    (SplineMesh|SetStartandEnd (Utilities|Array|Get(acopy) (Variables|Default|GetMeshes) _index) (.Location (Spline|GetLocationandTangentatSplinePoint _spline _index "World")) (.Tangent (Spline|GetLocationandTangentatSplinePoint _spline _index "World")) (.Location (Spline|GetLocationandTangentatSplinePoint _spline (+ _index 1) "World")) (.Tangent (Spline|GetLocationandTangentatSplinePoint _spline (+ _index 1) "World")) true :!class /Script/Engine.SplineMeshComponent)))

(fn GetSplineLastPointIndex
  (return (- (Spline|GetNumberOfSplinePoints (Variables|Default|GetSpline)) 1)))

(fn AddMeshSection
  (params (DebutPointIndex :type Integer))
  (bind _returnvalue (+ DebutPointIndex 1))
  (bind _spline (Variables|Default|GetSpline))
  (bind (_location _tangent) (Spline|GetLocationandTangentatSplinePoint _spline DebutPointIndex "World"))
  (bind (_location_2 _tangent_2) (Spline|GetLocationandTangentatSplinePoint _spline _returnvalue "World"))
  (bind _returnvalue_2 (AddComponent|AddSplineMeshComponent true))
  (Transformation|AttachComponentToComponent _returnvalue_2 (Variables|Default|GetTopScene) "None" "KeepRelative" "KeepRelative" "KeepRelative" true)
  (SplineMesh|SetStartandEnd _returnvalue_2 _location _tangent _location_2 _tangent_2 true :!class /Script/Engine.SplineMeshComponent)
  (Utilities|Array|Add (Variables|Default|GetMeshes) _returnvalue_2))