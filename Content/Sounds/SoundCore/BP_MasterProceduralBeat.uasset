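; Master procedural beat Blueprint that acts as a looping music clock, started on BeginPlay or with a debug P key.
; It converts BPM to a timer interval, and each tick updates signal, beat reset, bar and measure indexes at the master resolution.
; It then derives the root note and scale from the current bar and pushes bar number, scale and root note out through CallPushBeat.
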(event Custom|Play
  (bind _bpm64_inms (CallFunction|SetBpm (Variables|Master|Bpm|GetBpmInBeat)))
  (bind _output_get (Variables|Master|Bpm|SetBpm%20in%20Ms _bpm64_inms))
  (bind _returnvalue (Utilities|Time|SetTimerbyEvent (delegate Custom|Play%20the%20Beat) _output_get true))
  (Variables|Master|Refs|SetTimerReference _returnvalue))

(event Custom|Play%20the%20Beat
  (CallFunction|MasterBeatIndexes (Variables|PassByRef|MasterBeat|GetPBR_MasterSignalResolutionIndex) (Variables|Master|GetMasterResolution) (Variables|PassbyRef|MasterBeat|GetPBR_MasterBeatReset) (Variables|PassbyRef|MasterBeat|GetPBR_MasterBarNumber) (Variables|PassbyRef|MasterBeat|GetPBR_MasterMeasureNumber))
  (CallFunction|RootNoteandScale (Variables|PassbyRef|RootNote|GetPBR_FirstNoteRoot) (Variables|PassbyRef|MasterBeat|GetPBR_MasterBarNumber) (Variables|Default|GetBarModulo) (Variables|Default|GetScale) (Variables|PassbyRef|RootNote|GetPBR_MasterRootNote) "NewEnumerator4" (Variables|PassbyRef|RootNote|GetPBR_RootNoteSet))
  (Default|CallPushBeat (Variables|PassbyRef|MasterBeat|GetPBR_MasterBarNumber) (Variables|Default|GetScale) (Variables|PassbyRef|RootNote|GetPBR_MasterRootNote)))

(event EventBeginPlay
  (CallFunction|Play))

(event Input|KeyboardEvents|P
  (params (Key :type Key%20Structure))
  ;[1 1 1] Debug
  (:Pressed
    (CallFunction|Play)))

(fn ConstructionScript)