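; Musical actor that plays granular synth notes and kick samples in time with the procedural music beat.
; It binds to the first BP_MasterProceduralBeat's PushBeat, storing the root note and running BeatStepMatrix to decide which beats trigger.
; Triggered steps optionally rewind and fire the Granular synth or play a 2D kick.
; ModularSynth starts with a preset but receives no notes; the random-octave note is only printed for debugging.
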(event Custom|PushBeat
  (params (BarNumber :type Integer) (Scale :type Array%20of%20Floats%20%28single-precision%29) (RootNote :type Float%20%28single-precision%29))
  (Variables|Default|SetRootNote RootNote)
  (bind _notethru (CallFunction|BeatStepMatrix (Variables|Default|GetBeatResolution) (Variables|Default|GetStepSequencer) (Variables|Default|GetBeatShuffle) (Variables|Default|GetBeatRandom) (Variables|Default|GetCurrentStep) (Variables|Default|GetSignalResolutionIndex) (Variables|Default|GetBeat) (Variables|Default|GetBeatReset)))
  (if _notethru
    (Development|PrintString (Utilities|String|ToString(Float) RootNote))
    (CallFunction|Synth)
    (CallFunction|Kick)))

(event Custom|Synth
  (bind _granular (Variables|Default|GetGranular))
  (if (Variables|Default|GetPlaySynth)
    (Class|GranularSynth|SetPlayheadTime _granular 0.3 0.0 "FromBeginning")
    (Development|PrintString (Utilities|String|ToString(Float) (CallFunction|MakeNote (Math|Random|RandomIntegerinRange 4 7) (Variables|Default|GetRootNote))) true true "(R=0.000000,G=1.000000,B=0.015495,A=1.000000)")
    (Class|GranularSynth|Noteon (Variables|Default|GetGranular) 0.0 127 -1.0)
    (Development|PrintString (Utilities|String|Append (Utilities|String|ToString(Float) (Class|GranularSynth|GetCurrentPlayheadTime _granular)) "----" (Utilities|String|ToString(Float) (Class|GranularSynth|GetSampleDuration _granular))) true true "(R=1.000000,G=0.167867,B=0.000000,A=1.000000)")))

(event Custom|Kick
  (if (Variables|Default|GetPlay%20Kick)
    (Audio|PlaySound2D "/Game/Sounds/Waves/Drums/Kick/Kick_Standard_KP1_20.Kick_Standard_KP1_20")))

(event EventBeginPlay
  (bind _granular (Variables|Default|GetGranular))
  (bind _modularsynth (Variables|Default|GetModularSynth))
  (bind _outactors (Actor|GetAllActorsOfClass "/Game/Sounds/SoundCore/BP_MasterProceduralBeat.BP_MasterProceduralBeat_C"))
  (Variables|Default|SetMasterProceduralBeatActor (Utilities|Array|Get(acopy) _outactors))
  (EventDispatchers|BindEventtoPushBeat (Variables|Default|GetMasterProceduralBeatActor) (delegate Custom|PushBeat))
  (CallFunction|SetSynthPreset)
  (Components|Activation|Activate _modularsynth false)
  (CameraShake|Start _modularsynth)
  (Class|GranularSynth|SetSoundWave _granular "/Game/Sounds/Waves/OldWaves/piss.piss")
  (CameraShake|Start _granular)
  (Class|GranularSynth|SetGrainDuration _granular 1.0 "(X=500.000000,Y=500.000000)")
  (Class|GranularSynth|SetPlayheadTime _granular 5.0 0.0 "FromBeginning")
  (Development|PrintString (Utilities|String|ToString(Float) (Class|GranularSynth|GetCurrentPlayheadTime _granular)) true true "(R=1.000000,G=0.167867,B=0.000000,A=1.000000)")
  (Class|GranularSynth|SetGrainsPerSecond _granular 1.0)
  (Class|GranularSynth|SetPlaybackSpeed _granular 1.0)
  (Class|GranularSynth|SetGrainEnvelopeType _granular "Rectangular")
  (Class|GranularSynth|SetGrainProbability _granular 1.0)
  (Class|GranularSynth|SetGrainVolume _granular 1.0 "(X=1.000000,Y=1.000000)"))

(fn ConstructionScript)

(fn SetSynthPreset
  (params (SynthNumber :type Integer))
  (Class|ModularSynthComponent|SetSynthPreset (Variables|Default|GetModularSynth) (.Preset (Utilities|Struct|BreakModularSynthPresetBankEntry (Utilities|Array|Get(acopy) (Variables|/Script/Synthesis.ModularSynthPresetBank|GetPresets (Variables|Default|GetSynthPresets)) SynthNumber)))))