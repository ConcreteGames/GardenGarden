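; Music manager Blueprint that plays the master music event on begin play, can restart it, and supplies randomly chosen events for plants.
; Timeline beats from the master event pass through a FlipFlop, so CallMusicBeat fires on every other beat.
; ChooseEvent returns a random EventArray entry, limiting the first plant's pick to the first eight indices.
; ManageArray, marked unused, only triggers SetPlantMusicalEvent on the given actor.
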(event OnTimelineBeat(A_MasterMusicEvent)
  (params (Bar :type Integer) (Beat :type Integer) (Position :type Integer) (Tempo :type Float%20%28single-precision%29) (TimeSignatureUpper :type Integer) (TimeSignatureLower :type Integer))
  (Utilities|FlowControl|FlipFlop
    (:A
      (Default|CallMusicBeat))))

(event Custom|Manage%20Event%20Array
  (params (ReleasedEvent :type FMOD%20Event%20Object%20Reference) (ActorReferenced :type BP%20Plant%20Visual%20Parent%20Object%20Reference) (Destroy :type Boolean))
  ;[1 1 1] not used
  (Default|SetPlantMusicalEvent ActorReferenced))

(event Custom|RestartMusic
  (bind _a_mastermusicevent (Variables|Default|GetA_MasterMusicEvent))
  (Class|FMODAudioComponent|Stop _a_mastermusicevent)
  (Class|FMODAudioComponent|Play _a_mastermusicevent))

(event EventBeginPlay
  ;[1 1 1] BEGIN PLAY
  (Class|FMODAudioComponent|Play (Variables|Default|GetA_MasterMusicEvent)))

(fn ConstructionScript)

(fn ChooseEvent
  (if (Variables|Default|GetFirstPlant)
    (Variables|Default|SetRandomIntForEventSelection (Math|Random|RandomIntegerinRange 0 7))
    (Variables|Default|SetFirstPlant false)
    (else
      (Variables|Default|SetRandomIntForEventSelection (Math|Random|RandomIntegerinRange 0 (Utilities|Array|LastIndex (Variables|Default|GetEventArray))))))
  (for (_array_element _array_index) (Variables|Default|GetEventArray)
    (if (== _array_index (Variables|Default|GetRandomIntForEventSelection))
      (LocalVariables|SetChosenEvent _array_element)))
  (return (LocalVariables|GetChosenEvent) 0))