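; BP_Tiling is a construction-script Blueprint that lays out a grid of static mesh tiles around a central Cube.
; It scales the Cube horizontally by TileSize, then iterates X/Y offsets from ForEachReplication using DisplayDistance.
; Each non-origin offset gets a matching Static Mesh Component, spaced at TileSize times 100 units and stored in the Tiles array.
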(fn ConstructionScript
  (bind _tilesize (Variables|Default|GetTileSize))
  (bind _tilesize_2 (Variables|Default|GetTileSize))
  (bind _tilesize_3 (Variables|Default|GetTileSize))
  (bind _returnvalue (* _tilesize_2 1e+02))
  (Transformation|SetRelativeScale3D (Variables|Default|GetCube) (Math|Vector|MakeVector _tilesize _tilesize 1.0))
  (bind (_x _y) (Utilities|ForEachReplication (Variables|Default|GetDisplayDistance))
    (:LoopBody
      (if (not (and (== _x 0) (== _y 0)))
        (bind _returnvalue_2 (AddComponent|AddStaticMeshComponent false (Math|Transform|MakeTransform (Math|Vector|MakeVector (* _x _returnvalue) (* _y _returnvalue) 0.0) "0, 0, 0" (Math|Vector|MakeVector _tilesize_3 _tilesize_3 1.0))))
        (Utilities|Array|Add (Variables|Default|GetTiles) _returnvalue_2)))))