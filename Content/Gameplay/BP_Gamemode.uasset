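; Game mode that sets rendering console variables at begin play and drives plant-based milestones in a seed-and-plant game.
; A looping one-second timer gathers all BP_Plant actors and passes them to the event checks.
; A BP_Plant_Child2 starts music, and a plant with index 5 gives the hero low gravity and a higher jump.
; It spawns a seed at a TargetPoint when no plants or seeds exist and the hero holds none.
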(event Custom|CheckGameEvents
  (bind _outactors (Actor|GetAllActorsOfClass "/Game/Objects/Plants/BP_Plant.BP_Plant_C"))
  (CallFunction|PlayMusicatPlant2 _outactors)
  (CallFunction|SuperJumpandColoratPlant5 _outactors)
  (CallFunction|PopOneSeedifNoPlantNoSeed _outactors))

(event Custom|DebugSpawnSeed
  (params (Index :type Integer))
  (bind _outactors (Actor|GetAllActorsOfClass "/Script/Engine.TargetPoint"))
  (Game|SpawnActorfromClass "/Game/Objects/BP_Seed.BP_Seed_C" (Transformation|GetActorTransform (Utilities|Array|Get(acopy) _outactors)) "Undefined" 0 false Index true 0))

(event EventBeginPlay
  ;[0.07847 1 0] BEGIN PLAY
  (CallFunction|SetRendering)
  (Utilities|Time|SetTimerbyEvent (delegate Custom|CheckGameEvents) 1.0 true))

(fn ConstructionScript)

(fn PlayMusicatPlant2
  (params (Array :type Array%20of%20BP%20Plant%20Object%20References))
  (if (not (Variables|Default|GetChild2OK))
    (for _array_element Array
      (if (== (Utilities|GetClass _array_element) "/Game/Objects/Plants/BP_Plant_Child2.BP_Plant_Child2_C")
        (Utilities|FlowControl|DoOnce false
          (:Completed
            (Variables|Default|SetChild2OK true)
            (Audio|Components|Audio|Play (Variables|Default|GetAudio) 0.0)))))))

(fn SuperJumpandColoratPlant5
  (params (Array :type Array%20of%20BP%20Plant%20Object%20References))
  (if (not (Variables|Default|GetChild5OK))
    (for _array_element Array
      (if (== (Variables|/Game/Objects/Plants/BP_Plant.BP_Plant_C|GetPlantIndex _array_element) 5)
        (Utilities|FlowControl|DoOnce false
          (:Completed
            (Variables|Default|SetChild5OK false)
            (bind _asbp_hero_n (Utilities|Casting|CastToBP_HeroN (Game|Player|GetPlayerPawn 0)))
            (Variables|/Script/Engine.CharacterMovementComponent|SetGravityScale (Variables|/Script/Engine.Character|GetCharacterMovement _asbp_hero_n) 0.25)
            (Variables|/Script/Engine.CharacterMovementComponent|SetJumpZVelocity (Variables|/Script/Engine.Character|GetCharacterMovement _asbp_hero_n) 6e+02)))))))

(fn PopOneSeedifNoPlantNoSeed
  (params (PlantsArray :type Array%20of%20BP%20Plant%20Object%20References))
  (bind _outactors (Actor|GetAllActorsOfClass "/Game/Objects/BP_Seed.BP_Seed_C"))
  (bind _asbp_hero_n (Utilities|Casting|CastToBP_HeroN (Game|Player|GetPlayerPawn 0)))
  (if (Math|Boolean|ANDBoolean (not (Variables|/Game/Character/BP_HeroN.BP_HeroN_C|GetSeedIsInHand _asbp_hero_n)) (== (Utilities|Array|Length _outactors) 0) (== (Utilities|Array|Length PlantsArray) 0))
    ;[1 1 1] Pop 1st seed
    (bind _outactors_2 (Actor|GetAllActorsOfClass "/Script/Engine.TargetPoint"))
    (Game|SpawnActorfromClass "/Game/Objects/BP_Seed.BP_Seed_C" (Transformation|GetActorTransform (Utilities|Array|Get(acopy) _outactors_2)) "Undefined" 0 false 1 true 0)))

(fn SetRendering
  (Development|ExecuteConsoleCommand "r.ScreenPercentage 100")
  (Development|ExecuteConsoleCommand "r.vsynceditor 0")
  (Development|ExecuteConsoleCommand "r.vsync 0")
  (Development|ExecuteConsoleCommand "r.ViewDistanceScale 0.1")
  (Development|ExecuteConsoleCommand "r.PostProcessAAQuality 6")
  (Development|ExecuteConsoleCommand "sg.PostProcessQuality 0")
  (Development|ExecuteConsoleCommand "sg.ShadowQuality 3")
  (Development|ExecuteConsoleCommand "sg.TextureQuality 3")
  (Development|ExecuteConsoleCommand "sg.EffectsQuality 3")
  (Development|ExecuteConsoleCommand "r.DetailMode 2")
  (Development|ExecuteConsoleCommand "FoliageQuality 3"))