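; BP_PCont, by its name a player controller, provides debug hotkeys for profiling and game speed.
; F and G run the stat UnitGraph and stat fps console commands, while K and L start and stop stat file recording with a colored on-screen message.
; C, V and B set global time dilation to fast, normal and slow motion.
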(event EventBeginPlay)

(event EventTick
  (params (DeltaSeconds :type Float%20%28single-precision%29)))

(event Input|KeyboardEvents|F
  (params (Key :type Key%20Structure))
  (:Pressed
    (Development|ExecuteConsoleCommand "stat UnitGraph")))

(event Input|KeyboardEvents|C
  (params (Key :type Key%20Structure))
  (:Pressed
    (Utilities|Time|SetGlobalTimeDilation 2.0)))

(event Input|KeyboardEvents|V
  (params (Key :type Key%20Structure))
  (:Pressed
    (Utilities|Time|SetGlobalTimeDilation 1.0)))

(event Input|KeyboardEvents|B
  (params (Key :type Key%20Structure))
  (:Pressed
    (Utilities|Time|SetGlobalTimeDilation 0.5)))

(event Input|KeyboardEvents|G
  (params (Key :type Key%20Structure))
  (:Pressed
    (Development|ExecuteConsoleCommand "stat fps")))

(event Input|KeyboardEvents|K
  (params (Key :type Key%20Structure))
  (:Pressed
    (Development|ExecuteConsoleCommand "stat startfile")
    (Development|PrintString "START recording profiling" true true "(R=0.146088,G=1.000000,B=0.000000,A=1.000000)")))

(event Input|KeyboardEvents|L
  (params (Key :type Key%20Structure))
  (:Pressed
    (Development|ExecuteConsoleCommand "stat stopfile")
    (Development|PrintString "STOP recording profiling" true true "(R=1.000000,G=0.000000,B=0.000000,A=1.000000)")))

(fn ConstructionScript)