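; BP_HeroVisual is the hero's visual actor, showing the animated character and the seed it carries.
; The construction script adds a scaled seed static mesh and attaches it to the skeletal mesh's joint7 socket.
; Events switch between looping run and idle animations, move the actor with an XY offset while applying roll and yaw, and toggle seed visibility with an index-selected material.
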(event Custom|PlayAnimation
  (params (Run :type Boolean))
  (Components|Animation|PlayAnimation (Variables|Default|GetSkeletalMesh) (select Run "/Game/Character/HeroAnim/Run.Run" "/Game/Character/HeroAnim/Idle.Idle") true))

(event Custom|SetLocAndRot
  (params (NewLocation :type Vector) (NewRotation :type Rotator))
  (bind _offset (Variables|Default|GetOffset))
  (Transformation|SetActorLocationAndRotation (+ NewLocation (Math|Vector|MakeVector (.x _offset) (.y _offset) 0.0)) (Math|Rotator|MakeRotator (.roll NewRotation) 0.0 (.yaw NewRotation))))

(event Custom|SeeSeed
  (params (Visibility :type Boolean) (Index :type Integer))
  (bind _seed (Variables|Default|GetSeed))
  (Rendering|Material|SetMaterial _seed 1 (Utilities|Select :Index Index :Option%200 "/Game/Objects/Plants3D/Seed/M_Graine_1.M_Graine_1" :Option%201 "/Game/Objects/Plants3D/Seed/M_Graine_1.M_Graine_1" :Option%202 "/Game/Objects/Plants3D/Seed/M_Graine_2.M_Graine_2" :Option%203 "/Game/Objects/Plants3D/Seed/M_Graine_3.M_Graine_3" :Option%204 "/Game/Objects/Plants3D/Seed/M_Graine_4.M_Graine_4" :Option%205 "/Game/Objects/Plants3D/Seed/M_Graine_5.M_Graine_5"))
  (Rendering|SetVisibility _seed Visibility false))

(fn ConstructionScript
  (bind _returnvalue (AddComponent|AddStaticMeshComponent false (Math|Transform|MakeTransform "0,-1.000000,0.000000" "0.000000,0.000000,-90.000000" "0.006000,0.006000,0.006000")))
  (bind _output_get (Variables|Default|SetSeed _returnvalue))
  (Transformation|AttachComponentToComponent _output_get (Variables|Default|GetSkeletalMesh) "joint7" "KeepRelative" "KeepRelative" "KeepRelative" true))